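; WallSlideOpen is a sliding wall or door Blueprint with open and close functions for its static mesh.
; SlideDoorOpen offsets the mesh up 120 units in Z and SlideDoorClose offsets it down by the same amount, with debug prints.
; Each lerp has a fixed zero alpha, so movement is instant, and feeds a world-space position into SetRelativeLocation.
; The event graph is empty, so nothing here calls either function.
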(event EventBeginPlay)

(event Collision|EventActorBeginOverlap
  (params (OtherActor :type Actor%20Object%20Reference)))

(event EventTick
  (params (DeltaSeconds :type Float%20%28single-precision%29)))

(fn ConstructionScript)

(fn SlideDoorOpen
  (bind _staticmeshcomponent (Variables|Debug|GetStaticMeshComponent))
  (bind _returnvalue (Transformation|GetWorldLocation _staticmeshcomponent))
  (Development|PrintString "setting relative location")
  (Transformation|SetRelativeLocation (Variables|Debug|GetStaticMeshComponent) (Math|Vector|Lerp(Vector) (- _returnvalue "0, 0,-120.000000") _returnvalue 0.0) false false)
  (Development|PrintString "Door Open" true true "(R=1.000000,G=0.023286,B=0.000000,A=1.000000)" 4.0))

(fn SlideDoorClose
  (bind _staticmeshcomponent (Variables|Debug|GetStaticMeshComponent))
  (bind _returnvalue (Transformation|GetWorldLocation _staticmeshcomponent))
  (Development|PrintString "Setting relative location back")
  (Transformation|SetRelativeLocation (Variables|Debug|GetStaticMeshComponent) (Math|Vector|Lerp(Vector) (- _returnvalue "0, 0,120.000000") _returnvalue 0.0) false false)
  (Development|PrintString "Door Open"))