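; BP_SpeedBoost is a trigger pad that gives the player a temporary walk speed boost on overlap.
; When the player pawn enters the collision component while not crouching, CharBase's MaxWalkSpeed is set to the boost value, then to a reset value after a delay.
; A DoOnce gate limits this to one activation per entry and re-arms when the player leaves.
; Debug prints report the character name and the speed reset.
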(event OnComponentBeginOverlap(CollisionComponent)
  (params (OverlappedComponent :type Primitive%20Component%20Object%20Reference) (OtherActor :type Actor%20Object%20Reference) (OtherComp :type Primitive%20Component%20Object%20Reference) (OtherBodyIndex :type Integer) (bFromSweep :type Boolean) (SweepResult :type Hit%20Result%20Structure%20%28by%20ref%29))
  (bind _resetplayerspeed (Variables|Default|GetResetPlayerSpeed))
  ;[1 1 1] Pad Boost // when player enters zone, they get a temporary short speed boost.
  (if (== OtherActor (Game|Player|GetPlayerPawn 0))
    (Utilities|FlowControl|DoOnce false
      (:Completed
        (bind _aschar_base (Utilities|Casting|CastToCharBase (Game|GetPlayerCharacter 0)))
        (if (not (Variables|/Game/FirstPersonBP/Blueprints/CharBase.CharBase_C|GetIsCrouching? _aschar_base))
          (Development|PrintString (Utilities|GetDisplayName _aschar_base))
          (Variables|/Script/Engine.CharacterMovementComponent|SetMaxWalkSpeed (Variables|/Script/Engine.Character|GetCharacterMovement _aschar_base) (Variables|Default|GetPlayerSpeedBoost))
          (Utilities|FlowControl|Delay (Variables|Default|GetSpeedBoostTime))
          (Variables|/Script/Engine.CharacterMovementComponent|SetMaxWalkSpeed (Variables|/Script/Engine.Character|GetCharacterMovement _aschar_base) _resetplayerspeed)
          (Development|PrintString (Utilities|String|ToString(Float) _resetplayerspeed))
          (Development|PrintString "Walk Speed Set to Default" true true "(R=0.687500,G=0.000000,B=0.055091,A=1.000000)"))))))

(event OnComponentEndOverlap(CollisionComponent)
  (params (OverlappedComponent :type Primitive%20Component%20Object%20Reference) (OtherActor :type Actor%20Object%20Reference) (OtherComp :type Primitive%20Component%20Object%20Reference) (OtherBodyIndex :type Integer))
  (bind _resetplayerspeed (Variables|Default|GetResetPlayerSpeed))
  ;[1 1 1] Pad Boost // when player enters zone, they get a temporary short speed boost.
  (if (== OtherActor (Game|Player|GetPlayerPawn 0))
    (Utilities|FlowControl|DoOnce false) ; enters at Reset
  ))

(fn ConstructionScript)