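; Launchpad actor that launches the player character upward or along a set velocity and animates its mesh dipping and rising.
; A Box trigger flags when something is above the pad; player overlap then launches the CharBase after a short delay, with a brief relaunch lockout.
; Two timelines lerp mesh height down and back up behind a DoOnce, though both play-rate calls target the down timeline.
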(event OnComponentBeginOverlap(Box)
  (params (OverlappedComponent :type Primitive%20Component%20Object%20Reference) (OtherActor :type Actor%20Object%20Reference) (OtherComp :type Primitive%20Component%20Object%20Reference) (OtherBodyIndex :type Integer) (bFromSweep :type Boolean) (SweepResult :type Hit%20Result%20Structure%20%28by%20ref%29))
  ;[1 1 1] Triggers check if player is above launchpad
  (Variables|Default|SetChar%20above%20Launchpad? true))

(event OnComponentEndOverlap(Box)
  (params (OverlappedComponent :type Primitive%20Component%20Object%20Reference) (OtherActor :type Actor%20Object%20Reference) (OtherComp :type Primitive%20Component%20Object%20Reference) (OtherBodyIndex :type Integer))
  ;[1 1 1] Triggers check if player is above launchpad
  (Variables|Default|SetChar%20above%20Launchpad? false))

(event Collision|EventActorBeginOverlap
  (params (OtherActor :type Actor%20Object%20Reference))
  (bind _staticmeshcomponent (Variables|Debug|GetStaticMeshComponent))
  (bind _staticmeshcomponent_2 (Variables|Debug|GetStaticMeshComponent))
  (bind _returnvalue (Transformation|GetWorldLocation _staticmeshcomponent))
  (bind _returnvalue_2 (Transformation|GetWorldLocation _staticmeshcomponent_2))
  ;[1 1 1] Char Launch, if character is above pad.
  (if (== OtherActor (Game|Player|GetPlayerPawn 0))
    (if (Variables|Default|GetChar%20above%20Launchpad?)
      (if (not (Variables|Default|GetCharacterLaunched?))
        (Utilities|FlowControl|Sequence
          (:then_0
            (Utilities|FlowControl|Delay 0.2)
            (bind _aschar_base (Utilities|Casting|CastToCharBase OtherActor))
            (Character|LaunchCharacter _aschar_base (Variables|Default|GetPlayer%20Launch%20Velocity) false false)
            (Variables|Default|SetCharacterLaunched? true)
            (Utilities|FlowControl|Delay 1.0)
            (Variables|Default|SetCharacterLaunched? false))
          (:then_1
            ;;[1 1 1] Pad Down Animation
            (Utilities|FlowControl|DoOnce false :!label _label
              (:Completed
                (Components|Timeline|SetPlayRate (Variables|Default|GetJumpad%20Timeline) (/ 1.0 (Variables|Default|GetTime%20Seq%20JumpPad%20Down%20Animation)))
                (bind _scalar (Timeline|Jumpad%20Timeline PlayFromStart)
                  (:Update
                    (Development|PrintString "Pad Down")
                    (Transformation|SetRelativeLocation _staticmeshcomponent_2 (Math|Vector|MakeVector (.x _returnvalue_2) (.y _returnvalue_2) (Math|Float|Lerp (Variables|Default|GetJumpPad%20Start%20Pos) (Variables|Default|GetJumpPad%20Down%20Pos) _scalar)) false false)
                    (Development|PrintString "Pad going down")
                    ;;[1 1 1] Pad Up Animation
                    (Utilities|FlowControl|Delay 0.1)
                    (Components|Timeline|SetPlayRate (Variables|Default|GetJumpad%20Timeline) (/ 1.0 (Variables|Default|GetTime%20Seq%20JumpPad%20Up%20Animation)))
                    (bind _scalar_2 (Timeline|Timeline_0 PlayFromStart)
                      (:Update
                        (Development|PrintString "Pad Up" true true "(R=0.998654,G=1.000000,B=0.000000,A=1.000000)")
                        (Transformation|SetRelativeLocation _staticmeshcomponent (Math|Vector|MakeVector (.x _returnvalue) (.y _returnvalue) (Math|Float|Lerp (Variables|Default|GetJumpPad%20Down%20Pos) (Variables|Default|GetJumpPad%20Start%20Pos) _scalar_2)) false false)
                        (goto _label Reset)))))))))))))

(fn ConstructionScript)