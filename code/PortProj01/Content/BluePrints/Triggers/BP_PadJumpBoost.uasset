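; Jump boost pad trigger that launches the player character with a set velocity when it overlaps the pad while jumping.
; Tick polls the player's CharBase jump state, latching and debug-printing a flag.
; Actor overlap checks that flag and the live jump state, launches additively, clears the flag and resets its DoOnce.
; Collision component overlaps track an in-trigger flag, used only by a disconnected, delay-based launch variant.
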(event OnComponentBeginOverlap(CollisionComponent)
  (params (OverlappedComponent :type Primitive%20Component%20Object%20Reference) (OtherActor :type Actor%20Object%20Reference) (OtherComp :type Primitive%20Component%20Object%20Reference) (OtherBodyIndex :type Integer) (bFromSweep :type Boolean) (SweepResult :type Hit%20Result%20Structure%20%28by%20ref%29))
  ;[1 1 1] Triggers check if player is above launchpad
  (Variables|Default|SetCharacterInTrigger? true))

(event OnComponentEndOverlap(CollisionComponent)
  (params (OverlappedComponent :type Primitive%20Component%20Object%20Reference) (OtherActor :type Actor%20Object%20Reference) (OtherComp :type Primitive%20Component%20Object%20Reference) (OtherBodyIndex :type Integer))
  ;[1 1 1] Triggers check if player is above launchpad
  (Variables|Default|SetCharacterInTrigger? false))

(event EventTick
  (params (DeltaSeconds :type Float%20%28single-precision%29))
  (bind _aschar_base (Utilities|Casting|CastToCharBase (Game|GetPlayerCharacter 0)))
  (if (Variables|/Game/FirstPersonBP/Blueprints/CharBase.CharBase_C|GetIs%20Jumping? _aschar_base)
    (bind _output_get (Variables|Default|SetCharacterHasJumped? true))
    (Development|PrintString "Player BP Is JUMPING?" _output_get)))

(event Collision|EventActorBeginOverlap
  (params (OtherActor :type Actor%20Object%20Reference))
  ;[1 1 1] Char Launch, if character is above pad.
  (if (== OtherActor (Game|Player|GetPlayerPawn 0))
    (Utilities|FlowControl|Sequence
      (:then_0
        (if (Variables|Default|GetCharacterHasJumped?)
          (Utilities|FlowControl|Sequence
            (:then_0
              (bind _aschar_base (Utilities|Casting|CastToCharBase OtherActor))
              (if (Variables|/Game/FirstPersonBP/Blueprints/CharBase.CharBase_C|GetIs%20Jumping? _aschar_base)
                (Utilities|FlowControl|DoOnce false :!label _label
                  (:Completed
                    (Character|LaunchCharacter _aschar_base (Variables|Default|GetPlayerLaunchVelocity) false false)
                    (Variables|Default|SetCharacterHasJumped? true)
                    (Utilities|FlowControl|Sequence
                      (:then_0
                        (Variables|Default|SetCharacterHasJumped? false))))))))))
      (:then_1
        (goto _label Reset)))))

(fn ConstructionScript)