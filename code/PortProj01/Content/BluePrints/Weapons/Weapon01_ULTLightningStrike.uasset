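; Ultimate ability actor for Weapon01 that rains lightning strikes over an area, then destroys itself once the strike total reaches its maximum.
; A looping timer re-runs ULTSpawnStrikes, which spawns short-lived spawn-point actors at random points in a box sized by BoundingSphereCheck's radius, capped by level-wide count.
; CheckGroundLocation line-traces down from each point, and a Weapon01_LightningStrike spawns at the returned impact point.
; Debug prints, persistent trace drawing and an unused example trace remain.
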(event Custom|ULT%20Spawn%20Strikes
  (Utilities|Time|SetTimerbyEvent (delegate Custom|ULT%20Spawn%20Strikes) (Variables|Default|GetTimeBetweenStrikes) true)
  (Development|PrintString "ULT BEGINS")
  ;[1 1 1] Checks for the amount of ULT spawns allowed in level // Executes spawn code if less than max allowed
  (bind _outactors (Actor|GetAllActorsOfClass "/Game/BluePrints/Weapons/Weapon01_ULTSpawnPoints.Weapon01_ULTSpawnPoints_C"))
  (if (< (Utilities|Array|Length _outactors) (Variables|Default|GetMaxULTspawns))
    ;[1 1 1] Condition is true, if the current # of lightning stikes is less than the ULT strike Total. // When the ULT strike total reaches max strikes, this actor is destroyed
    (if (< (Utilities|Array|Length (Variables|Default|GetULT_StikeTotal)) (Variables|Default|GetMaxStrikesForULT))
      ;[1 1 1] Spawn Lightning stike spawn BP at a random points withing the bounding sphere, then checks for ground location below each spawn point and spawns lightning strike at the ground location // add to ULT Stike Total (array).
      (bind _returnvalue (Game|SpawnActorfromClass "/Game/BluePrints/Weapons/Weapon01_ULTSpawnPoints.Weapon01_ULTSpawnPoints_C" (Math|Conversions|ToTransform(Vector) (Math|Random|RandomPointinBoundingBox (Transformation|GetWorldLocation (Variables|Default|GetULT%20Spawn)) (Math|Conversions|ToVector(Float) (Components|Sphere|GetScaledSphereRadius (Variables|Default|GetBoundingSphereCheck))))) "Undefined" 0 0))
      (Actor|SetLifeSpan _returnvalue (Variables|Default|GetULTspawn%20Lifespan))
      (bind _impactpoint (CallFunction|CheckGroundLocation (Variables|/Game/BluePrints/Weapons/Weapon01_ULTSpawnPoints.Weapon01_ULTSpawnPoints_C|GetULT%20Spawn _returnvalue)))
      (bind _returnvalue_2 (Game|SpawnActorfromClass "/Game/BluePrints/Weapons/Weapon01_LightningStrike.Weapon01_LightningStrike_C" (Math|Conversions|ToTransform(Vector) _impactpoint) "Undefined" 0 0))
      (bind _returnvalue_3 (Utilities|Array|Add (Variables|Default|GetULT_StikeTotal) _returnvalue_2))
      ;[1 1 1] Debug
      (Development|PrintString (Utilities|String|ToString(Integer) _returnvalue_3) true true "(R=0.000000,G=0.660000,B=1.000000,A=1.000000)" 1e+01)
      (Development|PrintString "Lightning Strike Count is =" true true "(R=1.000000,G=0.000000,B=0.049434,A=1.000000)" 1e+01)
      (else
        (Actor|DestroyActor)))))

(event EventBeginPlay
  (bind _boundingspherecheck (Variables|Default|GetBoundingSphereCheck))
  ;[1 1 1] Begins ULT event and then moves the bounding sphere collision for the ult // betters positions the collision space that acts as a bounding box
  (CallFunction|ULTSpawnStrikes)
  (Transformation|SetRelativeLocation _boundingspherecheck (+ (Transformation|GetWorldLocation _boundingspherecheck) "0.000000,0.000000,1000.000000") false false))

(fn ConstructionScript)

(fn CheckGroundLocation
  (params (GetWorldLocation :type Scene%20Component%20Object%20Reference))
  (bind _returnvalue (Transformation|GetWorldLocation GetWorldLocation))
  (bind (_outhit _returnvalue_2) (Collision|LineTraceByChannel _returnvalue (+ _returnvalue (* (Math|Vector|GetReflectionVector "0, 0,-100.000000" "0, 0, 0") (Variables|Default|GetLineTraceToGroundLengthCheck))) "TraceTypeQuery1" false 0 "Persistent"))
  (if _returnvalue_2
    (Utilities|FlowControl|Sequence
      (:then_0
        (return (.ImpactPoint (Collision|BreakHitResult _outhit))))
      (:then_1
        (Variables|Default|SetGroundLocation (.Location (Collision|BreakHitResult _outhit)))))
    (else
      (return (.ImpactPoint (Collision|BreakHitResult _outhit))))))