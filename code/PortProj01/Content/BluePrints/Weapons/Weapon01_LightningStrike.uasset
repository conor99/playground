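; Lightning strike weapon actor that, after a configurable delay on spawn, hits enemies inside its overlap check area.
; It plays two attached lightning particle effects, damages each overlapping SimpleAI through TakeDamage30, and adds to the player character's ultimate percentage per enemy hit.
; It also spawns an Explosion_RadialForce actor at the strike point and destroys itself six seconds after BeginPlay.
; An unconnected line trace example remains in the graph.
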(event EventBeginPlay
  (Utilities|FlowControl|Sequence
    (:then_0
      ;[1 1 1] Delays Lightning Strike after the enemy check is spawned
      (Utilities|FlowControl|Delay (Variables|Default|GetLighting%20Strike%20Delay))
      (Utilities|FlowControl|Sequence
        (:then_0
          ;[1 1 1] Executes spawn emitter and deals damage to each enemy overlapping enemy check collision
          (Effects|SpawnEmitterAttached (Variables|Default|GetParticle_LightningOpt01) (Variables|Default|GetLightningSpawn) "None" "0, 0, 0" "0, 0, 0" (Variables|Default|GetParticleScale))
          (Effects|SpawnEmitterAttached (Variables|Default|GetParticle_LightningOpt02) (Variables|Default|GetLightningSpawn) "None")
          (Utilities|FlowControl|Sequence
            (:then_0
              (for _array_element (Collision|GetOverlappingActors (Variables|Default|GetEnemyOverlappingCheck) (Variables|Default|GetEnemyClass) :!class /Script/Engine.PrimitiveComponent)
                ;;[1 0.09258 0.07268] Will be removed at some point and add take damage for player characters
                (bind _assimple_ai (Utilities|Casting|CastToSimpleAI _array_element))
                (Default|TakeDamage30% _assimple_ai)
                (bind _aschar_base (Utilities|Casting|CastToCharBase (Game|GetPlayerCharacter 0)))
                (Default|AddValuetoULTpercentage _aschar_base)))
            (:then_1
              (Game|SpawnActorfromClass "/Game/BluePrints/Explosion_RadialForce.Explosion_RadialForce_C" (Transformation|GetWorldTransform (Variables|Default|GetLightningSpawn)) "AlwaysSpawn" 0 0))))))
    (:then_1
      ;[1 1 1] Destroys object after X seconds
      (Utilities|FlowControl|Delay 6.0)
      (Actor|DestroyActor))))

(fn ConstructionScript)